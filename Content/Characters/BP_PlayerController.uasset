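; Player controller that toggles the pause menu and the game's paused state from the IA_PauseGame input action.
; On each press it removes the existing menu widget or creates a WB_PauseMenuUI through DisplayPauseMenu and adds it to the viewport.
; It then checks whether the game is paused, either unpausing, hiding the mouse and clearing the widget reference, or pausing and showing the mouse.
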(event Input|EnhancedActionEvents|EnhancedInputActionIA_PauseGame
  (params (ActionValue :type Boolean) (ElapsedSeconds :type Float%20%28double-precision%29) (TriggeredSeconds :type Float%20%28double-precision%29) (InputAction :type Input%20Action%20Object%20Reference :default "/Game/Characters/Inputs/IA_PauseGame.IA_PauseGame"))
  ;[0.15 0.15 0.15 0.5] PauseGame
  (:Started
    (bind _wb_pausemenuui (Variables|Default|GetWB_PauseMenuUI)
      (:then
        (Widget|RemovefromParent _wb_pausemenuui))
      (:else
        (CallFunction|DisplayPauseMenu)))
    (if (Game|IsGamePaused)
      (Variables|Default|SetWB_PauseMenuUI 0)
      (CallFunction|HideMouse)
      (Game|SetGamePaused false)
      (else
        (CallFunction|ShowMouse)
        (Game|SetGamePaused true)))))

(event EventBeginPlay)

(event EventTick
  (params (DeltaSeconds :type Float%20%28single-precision%29)))

(fn ConstructionScript)

(fn DisplayPauseMenu
  (bind _returnvalue (UserInterface|CreateWidget "/Game/UI/WB_PauseMenuUI.WB_PauseMenuUI_C"))
  (bind _output_get (Variables|Default|SetWB_PauseMenuUI _returnvalue))
  (UserInterface|Viewport|AddtoViewport _output_get 0))