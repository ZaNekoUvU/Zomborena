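; Pistol weapon Blueprint that handles firing and switching to the pistol from the Toaster.
; Shoot extends the parent's Shoot with a ShotTrace over the weapon's Range.
; ShootWeapon sets the firing flag, executes a "Shooting" console command, plays a 2D gunshot sound and calls PistolShoot.
; SwitchtoPistol swaps visibility by showing the pistol actor and hiding the Toaster actor.
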(event EventShootWeapon
  (Variables|Default|SetFiringWeapon true)
  (Development|ExecuteConsoleCommand "Shooting" 0)
  (Audio|PlaySound2D "/Game/Characters/single-pistol-gunshot-33-37187.single-pistol-gunshot-33-37187" 0.1 1.0 0.0 0 0)
  (CallFunction|PistolShoot))

(event EventSwitchtoPistol
  (params (Pistol :type Base%20Weapon%20BP%20Object%20Reference) (Toaster :type Base%20Weapon%20BP%20Object%20Reference))
  (Rendering|SetActorHiddenInGame Pistol false)
  (Rendering|SetActorHiddenInGame Toaster true))

(event EventShoot
  (|CallParentFunction)
  (CallFunction|ShotTrace (Variables|Default|GetRange)))

(fn ConstructionScript
  (|CallParentFunction))