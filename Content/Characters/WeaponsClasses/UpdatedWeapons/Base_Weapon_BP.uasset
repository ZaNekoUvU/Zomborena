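; Base weapon Blueprint for the player's guns, providing hitscan shooting and a partial weapon switch, with most other events and functions left as stubs.
; ShotTrace and ToasterShoot trace from the player camera, applying impulse and damage with persistent debug lines; ShotTrace ignores its Range input.
; UpdatedSwitchWeapon hides the previous weapon and clears CurrentWeapon.
; Older pistol/toaster switching, list cycling and ammo-based firing remain as disconnected nodes.
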(event Custom|ShotTrace
  (params (Range :type Float%20%28double-precision%29))
  (bind _asplayer_blueprint (Utilities|Casting|CastToPlayerBlueprint (Game|GetPlayerCharacter 0)))
  (bind _outhit (Collision|LineTraceByChannel (Transformation|GetWorldLocation (Variables|/Game/Characters/PlayerBlueprint.PlayerBlueprint_C|GetCamera _asplayer_blueprint)) (+ (Transformation|GetWorldLocation (Variables|/Game/Characters/PlayerBlueprint.PlayerBlueprint_C|GetCamera _asplayer_blueprint)) (* (Math|Vector|GetForwardVector (Transformation|GetWorldRotation (Variables|/Game/Characters/PlayerBlueprint.PlayerBlueprint_C|GetCamera _asplayer_blueprint))) 1.5e+03)) "TraceTypeQuery1" false 0 "Persistent"))
  (Physics|AddImpulseatLocation (.HitComponent (Collision|BreakHitResult _outhit)) "500.000000,500.000000,500.000000" (.Location (Collision|BreakHitResult _outhit)) "None")
  (Game|Damage|ApplyDamage (.HitActor (Collision|BreakHitResult _outhit)) 3.0 0 0))

(event Custom|Shoot)

(event EventShootWeapon)

(event EventSwitchWeaponList
  (params (ChildActorRef :type Child%20Actor%20Component%20Object%20Reference)))

(event EventSwitchtoToaster
  (params (Pistol%20 :type Base%20Weapon%20BP%20Object%20Reference) (Toaster :type Base%20Weapon%20BP%20Object%20Reference)))

(event EventSwitchtoPistol
  (params (Pistol :type Base%20Weapon%20BP%20Object%20Reference) (Toaster :type Base%20Weapon%20BP%20Object%20Reference)))

(event EventUpdatedSwitchWeapon
  (params (char_Ref :type Player%20Blueprint%20Object%20Reference) (Curr_Wea_Ref :type Base%20Weapon%20BP%20Object%20Reference) (Weapon_Ref :type Base%20Weapon%20BP%20Class%20Reference) (Prev_Wea_Ref :type Base%20Weapon%20BP%20Object%20Reference))
  (Development|PrintString "Switch")
  (Development|PrintString (Utilities|GetClassDisplayName Weapon_Ref))
  (Rendering|SetActorHiddenInGame Prev_Wea_Ref true)
  (Variables|Default|SetcurrentWeapon 0))

(fn ConstructionScript)

(fn ToasterShoot
  (bind _asplayer_blueprint (Utilities|Casting|CastToPlayerBlueprint (Components|GetOwner)))
  (bind _outhit (Collision|LineTraceByChannel (Transformation|GetWorldLocation (Variables|/Game/Characters/PlayerBlueprint.PlayerBlueprint_C|GetCamera _asplayer_blueprint)) (+ (Transformation|GetWorldLocation (Variables|/Game/Characters/PlayerBlueprint.PlayerBlueprint_C|GetCamera _asplayer_blueprint)) (* (Math|Vector|GetForwardVector (Transformation|GetWorldRotation (Variables|/Game/Characters/PlayerBlueprint.PlayerBlueprint_C|GetCamera _asplayer_blueprint))) 1.5e+03)) "TraceTypeQuery1" false 0 "Persistent"))
  (Physics|AddImpulseatLocation (.HitComponent (Collision|BreakHitResult _outhit)) "500.000000,500.000000,500.000000" (.Location (Collision|BreakHitResult _outhit)) "None")
  (Game|Damage|ApplyDamage (.HitActor (Collision|BreakHitResult _outhit)) 12.0 0 0))

(fn PistolShoot
  (bind _asplayer_blueprint (Utilities|Casting|CastToPlayerBlueprint (Game|GetPlayerCharacter 0))))

(fn SwitchWeapon
  (params (PlayerCharacterRef :type Player%20Blueprint%20Object%20Reference) (Current_Weapon_Ref :type Base%20Weapon%20BP%20Object%20Reference) (Weapon :type Base%20Weapon%20BP%20Class%20Reference))
  (return 0))

(fn UpdateCurrentWeapon
  (return 0))