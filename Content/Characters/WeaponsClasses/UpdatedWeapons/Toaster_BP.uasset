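; Toaster weapon Blueprint that handles ammo-limited shooting and the visual swap from the pistol.
; ShootWeapon spends ammo, plays a gunshot and calls ToasterShoot, or plays a dry-fire sound when empty.
; Each shot sets ShootDelay, so the next call fires nothing and clears the flag one second later.
; SwitchtoToaster shows the toaster and hides the pistol; an ammo text update is left unwired.
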(event EventSwitchtoToaster
  (params (Pistol%20 :type Base%20Weapon%20BP%20Object%20Reference) (Toaster :type Base%20Weapon%20BP%20Object%20Reference))
  (Rendering|SetActorHiddenInGame Toaster false)
  (Rendering|SetActorHiddenInGame Pistol%20 true))

(event EventShootWeapon
  (if (Variables|Default|GetShootDelay)
    (Variables|Default|SetFiringWeapon false)
    (Development|ExecuteConsoleCommand "Stop Shooting" 0)
    (Utilities|FlowControl|Delay 1.0)
    (Variables|Default|SetShootDelay false)
    (else
      (bind _output_get (Variables|Default|SetToasterAmmo (Variables|Default|GetToasterAmmo)))
      (if (> _output_get 0)
        (bind _output_get_2 (Variables|Default|SetToasterAmmo (Variables|Default|GetToasterAmmo)))
        (Variables|Default|SetToasterAmmo (- _output_get_2 1))
        (Variables|Default|SetFiringWeapon true)
        (Development|ExecuteConsoleCommand "Shooting" 0)
        (Audio|PlaySound2D "/Game/Characters/single-pistol-gunshot-33-37187.single-pistol-gunshot-33-37187" 0.1 1.0 0.0 0 0)
        (CallFunction|ToasterShoot)
        (Variables|Default|SetShootDelay true)
        (else
          (Audio|PlaySound2D "/Game/Characters/empty-gun-shot-6209.empty-gun-shot-6209" 1.0 1.0 0.0 0 0))))))

(fn ConstructionScript
  (|CallParentFunction))