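; Weapon Blueprint for a pistol and an ammo-limited Toaster gun, with its fire events left empty and the firing logic disconnected.
; That unwired logic branches on HasPistol, handling sounds, console commands, shot delay, Toaster ammo and HUD text.
; ToasterShoot line-traces from the owning player's camera, applying impulse and damage with persistent debug drawing.
; PistolShoot only casts the player character; its similar, lower-damage trace is also disconnected.
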(event Custom|ShootPistol
  (params (Fire :type Player%20Blueprint%20Class%20Reference)))

(event EventShootWeapon
  ;[0.15 0.15 0.15 0.5] Fire
)

(fn ConstructionScript)

(fn ToasterShoot
  (bind _asplayer_blueprint (Utilities|Casting|CastToPlayerBlueprint (Components|GetOwner)))
  (bind _outhit (Collision|LineTraceByChannel (Transformation|GetWorldLocation (Variables|/Game/Characters/PlayerBlueprint.PlayerBlueprint_C|GetCamera _asplayer_blueprint)) (+ (Transformation|GetWorldLocation (Variables|/Game/Characters/PlayerBlueprint.PlayerBlueprint_C|GetCamera _asplayer_blueprint)) (* (Math|Vector|GetForwardVector (Transformation|GetWorldRotation (Variables|/Game/Characters/PlayerBlueprint.PlayerBlueprint_C|GetCamera _asplayer_blueprint))) 1.5e+03)) "TraceTypeQuery1" false 0 "Persistent"))
  (Physics|AddImpulseatLocation (.HitComponent (Collision|BreakHitResult _outhit)) "500.000000,500.000000,500.000000" (.Location (Collision|BreakHitResult _outhit)) "None")
  (Game|Damage|ApplyDamage (.HitActor (Collision|BreakHitResult _outhit)) 12.0 0 0))

(fn PistolShoot
  (bind _asplayer_blueprint (Utilities|Casting|CastToPlayerBlueprint (Game|GetPlayerCharacter 0))))